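; Padlock test interactable that shows a PIN entry widget when the player interacts with it up close.
; A box trigger tracks whether the first-person character is in range, gating the Interact event.
; Interacting creates a new WB_PinWidget and switches to Game and UI input with mouse cursor and click events.
; Leaving the box removes the widget and restores game-only input.
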(event `/Game/Blueprints/Interfaces/BPI_InteractionInterface.Interact`
  (bind _returnvalue (`GameplayStatics.GetPlayerController` 0))
  (if (`self.IsCloseEnough`)
    (bind _returnvalue_2 (`|CreateWidget` "/Game/Puzzles/WB_PinWidget.WB_PinWidget_C"))
    (`UserWidget.AddToViewport` _returnvalue_2 0)
    (`WidgetBlueprintLibrary.SetInputMode_GameAndUIEx` _returnvalue null)
    (set `PlayerController.bEnableClickEvents` true _returnvalue)
    (set `PlayerController.bShowMouseCursor` true _returnvalue)))

(event `self.Box.OnComponentBeginOverlap`
  (params (OverlappedComponent :type "PrimitiveComponent Object Reference") (OtherActor :type "Actor Object Reference") (OtherComp :type "PrimitiveComponent Object Reference") (OtherBodyIndex :type Integer) (bFromSweep :type Boolean) (SweepResult :type "HitResult Structure (by ref)"))
  (cast `/Game/FirstPerson/Blueprints/BP_FirstPersonCharacter` OtherActor)
  (set `self.IsCloseEnough` true))

(event `self.Box.OnComponentEndOverlap`
  (params (OverlappedComponent :type "PrimitiveComponent Object Reference") (OtherActor :type "Actor Object Reference") (OtherComp :type "PrimitiveComponent Object Reference") (OtherBodyIndex :type Integer))
  (bind _returnvalue (`GameplayStatics.GetPlayerController` 0))
  (cast `/Game/FirstPerson/Blueprints/BP_FirstPersonCharacter` OtherActor)
  (`Widget.RemoveFromParent` (stale `/Game/Blueprints/Interfaces/BPI_InteractionInterface.Interact` _returnvalue_2))
  (`WidgetBlueprintLibrary.SetInputMode_GameOnly` _returnvalue)
  (set `PlayerController.bEnableClickEvents` false _returnvalue)
  (set `PlayerController.bShowMouseCursor` false _returnvalue)
  (set `self.IsCloseEnough` false))

(fn `UserConstructionScript`)